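; Automatic gearbox component for a car that picks gears from engine RPM, speed, throttle and brake.
; Update shifts up or down at RPM thresholds, and each change completes after a timed delay that sets the gear ratio.
; ToWheel and ToEngine convert torque, velocity and inertia through that ratio.
; Auto-reverse selects first on throttle from neutral or reverse, but braking only reaches neutral because a hard-coded branch blocks reverse.
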(fn `GetGearIndex`
  (returns (Value :type Integer))
  (return (`self.GearIndex`)))

(fn `GetGearRatio`
  (returns (Value :type "Float (double-precision)"))
  (return (`self.GearRatio`)))

(fn `GetIsGearChangeInProgress`
  (returns (Value :type Boolean))
  (return (`self.IsGearChangeInProgress`)))

(fn `ShiftGearByIndex`
  (params (Index :type Integer))
  (if (and (>= Index -1) (<= Index (`KismetArrayLibrary.Array_Length` (`self.GearRatioArray`))))
    (set `self.NextGearIndex` Index)
    (set `self.IsGearChangeInProgress` true)
    (set `self.ElapsedTime` 0.0)))

(fn `ShiftGearCallback`
  (`|ExecutionSequence`
    (:`then_0`
      (bind _output_get (set `self.GearIndex` (`self.NextGearIndex`)))
      (if (== _output_get -1)
        (set `self.GearRatio` (`self.ReverseGearRatio`))
        (elif (== (`self.GearIndex`) 0)
          (set `self.GearRatio` 0.0)
          (else
            (set `self.GearRatio` (`|GetArrayItem` (`self.GearRatioArray`) (`self.GearIndex`)))))))
    (:`then_1`
      (set `self.IsGearChangeInProgress` false))))

(fn `ShiftGearDown`
  (if (> (`self.GearIndex`) 1)
    (set `self.NextGearIndex` (- (`self.GearIndex`) 1))
    (set `self.IsGearChangeInProgress` true)
    (set `self.ElapsedTime` 0.0)))

(fn `ShiftGearUp`
  (bind _gearindex (`self.GearIndex`))
  (if (< _gearindex (- (`KismetArrayLibrary.Array_Length` (`self.GearRatioArray`)) 1))
    (set `self.NextGearIndex` (+ _gearindex 1))
    (set `self.IsGearChangeInProgress` true)
    (set `self.ElapsedTime` 0.0)))

(fn `ToEngine`
  (params (InVelocity :type "Float (double-precision)") (InIntertia :type "Float (double-precision)"))
  (returns (OutVelocity :type "Float (double-precision)") (OutInertia :type "Float (double-precision)"))
  (bind _gearratio (`self.GearRatio`))
  (if (!= _gearratio 0.0)
    (return (/ InVelocity _gearratio) (* InIntertia (* _gearratio _gearratio)))
    (else
      (return 0.0 0.0))))

(fn `ToWheel`
  (params (InTorque :type "Float (double-precision)"))
  (returns (OutTorque :type "Float (double-precision)"))
  (return (* InTorque (`self.GearRatio`))))

(fn `Update`
  (params (InDeltaTime :type "Float (double-precision)") (InEngineRPM :type "Float (double-precision)") (InCarForwardSpeedMPS :type "Float (double-precision)") (InThrottle :type "Float (double-precision)") (InBrake :type "Float (double-precision)"))
  (`|ExecutionSequence`
    (:`then_0`
      (set `self.DeltaTime` InDeltaTime)
      (set `self.EngineRPM` InEngineRPM)
      (set `self.CarForwardSpeedMPS` InCarForwardSpeedMPS)
      (set `self.ThrottleInput` InThrottle)
      (set `self.BrakeInput` InBrake)
      (`self.UpdateTimer`)
      (if (`self.IsAutoGearShift`)
        (if (not (`self.IsGearChangeInProgress`))
          (if (> (`self.EngineRPM`) (`self.ShiftUpRPM`))
            (if (< (`self.GearIndex`) (- (`KismetArrayLibrary.Array_Length` (`self.GearRatioArray`)) 1))
              (`self.ShiftGearUp`))))))
    (:`then_1`
      (if (`self.IsAutoGearShift`)
        (if (not (`self.IsGearChangeInProgress`))
          (if (< (`self.EngineRPM`) (`self.ShiftDownRPM`))
            (if (> (`self.GearIndex`) 1)
              (`self.ShiftGearDown`))))))
    (:`then_2`
      (if (`self.IsAutoReverse`)
        (if (> (`self.BrakeInput`) 0.1)
          (if (< (`self.CarForwardSpeedMPS`) 0.5)
            (if true
              (`self.ShiftGearByIndex` 0)
              (elif (== (`self.GearIndex`) 0)
                (`self.ShiftGearByIndex` -1)))))))
    (:`then_3`
      (if (`self.IsAutoReverse`)
        (if (> (`self.ThrottleInput`) 0.1)
          (if (<= (`self.GearIndex`) 0)
            (`self.ShiftGearByIndex` 1)))))))

(fn `UpdateTimer`
  (if (`self.IsGearChangeInProgress`)
    (bind _output_get (set `self.ElapsedTime` (+ (`self.ElapsedTime`) (`self.DeltaTime`))))
    (if (>= _output_get (`self.GearShiftTime`))
      (`self.ShiftGearCallback`))))