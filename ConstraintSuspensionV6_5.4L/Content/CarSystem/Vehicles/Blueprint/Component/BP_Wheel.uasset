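; Custom wheel component for an AdvancedVehiclePawn that simulates tire physics through an externally called Update with drive, brake and steering inputs.
; It integrates spin and lock-up, then line-traces from the hub, treating the tire as a radial spring-damper.
; Slip, static and sliding friction are clamped to a friction circle and applied to the body.
; Longitudinal force feeds back as reaction torque; pneumatic trail yields aligning torque Mz.
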(event `self.ReceiveBeginPlay`
  (`self.UpdateInertia`)
  (bind _asadvanced_vehicle_pawn (cast `AdvancedVehiclePawn` (`self.GetOwner`)))
  (set `self.AdvancedVehiclePawn` _asadvanced_vehicle_pawn))

(fn `ApplyForces`
  (if (and (`KismetSystemLibrary.IsValid` (`self.Primitive`)) (`KismetSystemLibrary.IsValid` (`self.AdvancedVehiclePawn`)))
    (`AdvancedVehiclePawn.AddForceAtLocation` (`self.AdvancedVehiclePawn`) (`self.Primitive`) (* (`self.TireFzVec`) 100.0) (`.ImpactPoint` (`GameplayStatics.BreakHitResult` (`self.HitResult`))) false)
    (`AdvancedVehiclePawn.AddForceAtLocation` (`self.AdvancedVehiclePawn`) (`self.Primitive`) (* (`self.TireFrictionForceVec`) 100.0) (.location (`self.HubWorldTransform`)) false)))

(fn `ApplyTorque`
  (bind _wheelangularvelocity (`self.WheelAngularVelocity`))
  (bind _returnvalue (`KismetMathLibrary.SignOfFloat` _wheelangularvelocity))
  (bind _returnvalue_2 (+ _wheelangularvelocity (* (* (`KismetMathLibrary.Abs` (`self.BrakeTorque`)) _returnvalue -1.0) (`self.WheelInertiaInversed`) (`self.Delta Time`))))
  (set `self.WheelAngularVelocity` (+ (`self.WheelAngularVelocity`) (* (+ (`self.DriveTorque`) (`self.ReactionTorque`)) (`self.WheelInertiaInversed`) (`self.Delta Time`))))
  (if (== (`KismetMathLibrary.SignOfFloat` _returnvalue_2) _returnvalue)
    (set `self.WheelAngularVelocity` _returnvalue_2)
    (set `self.IsLocked` false)
    (else
      (set `self.WheelAngularVelocity` 0.0)
      (set `self.IsLocked` true))))

(fn `GetMz`
  (returns (Value :type "Float (double-precision)"))
  (return (`self.Mz`)))

(fn `GetTireRadialForce`
  (set `self.TireFz` (`KismetMathLibrary.FMax` (+ (* (`KismetMathLibrary.SafeDivide` (- (`self.TireCompressZ`) (`self.TireCompressZPrev`)) (`self.Delta Time`)) (`self.TireRadialDamping`)) (* (`self.TireCompressZ`) (`self.TireRadialStiffness`)))))
  (set `self.TireFzVec` (* (`.ImpactNormal` (`GameplayStatics.BreakHitResult` (`self.HitResult`))) (`self.TireFz`)))
  (set `self.TireCompressZPrev` (`self.TireCompressZ`))
  (set `self.MassPerWheel` (/ (`self.TireFz`) 9.8)))

(fn `GetWheelAngularVelocity`
  (returns (NewParam :type "Float (double-precision)"))
  (return (`self.WheelAngularVelocity`)))

(fn `GetWheelInertia`
  (returns (Value :type "Float (double-precision)"))
  (return (`self.WheelInertia`)))

(fn `GetWheelPitchAngle`
  (returns (Value :type "Float (double-precision)"))
  (return (`self.WheelPitchAngle`)))

(fn `GetWheelSteeringAngle`
  (returns (Value :type "Float (double-precision)"))
  (return (`self.SteeringAngle`)))

(fn `SetBody`
  (params (Primitive :type "PrimitiveComponent Object Reference"))
  (set `self.Primitive` Primitive))

(fn `TireModelGetForce`
  (bind (_slidingfriction_x _slidingfriction_y) (`KismetMathLibrary.BreakVector` (`self.SlidingFriction`)))
  (bind _slidingfriction_x_2 (`KismetMathLibrary.BreakVector` (`self.SlidingFriction`)))
  (bind _advancedvehiclepawn (`self.AdvancedVehiclePawn`))
  (bind _maxforce (`self.MaxForce`))
  (bind _tireforceunclamped (`self.TireForceUnclamped`))
  (bind _maxforce_2 (`self.MaxForce`))
  (bind _contactpatchrotation (`self.ContactPatchRotation`))
  (bind (_bblockinghit _binitialoverlap _time _distance _location _impactpoint _normal _impactnormal _physmat _hitactor _hitcomponent) (`GameplayStatics.BreakHitResult` (`self.HitResult`)))
  (bind (_bblockinghit_2 _binitialoverlap_2 _time_2 _distance_2 _location_2 _impactpoint_2 _normal_2 _impactnormal_2) (`GameplayStatics.BreakHitResult` (`self.HitResult`)))
  (bind _rotation (.rotation (`self.HubWorldTransform`)))
  (set `self.MaxForce` (* (`self.Mu`) (`self.TireFz`)))
  (if (and (`KismetSystemLibrary.IsValid` (`self.Primitive`)) (`KismetSystemLibrary.IsValid` (`self.AdvancedVehiclePawn`)) (`KismetSystemLibrary.IsValid` _hitcomponent))
    (bind _returnvalue (`AdvancedVehiclePawn.GetLinearVelocityAtPoint` _advancedvehiclepawn (`self.Primitive`) _impactpoint))
    (bind _returnvalue_2 (`AdvancedVehiclePawn.GetLinearVelocityAtPoint` _advancedvehiclepawn _hitcomponent _impactpoint))
    (bind _output_get (set `self.ContactPatchRotation` (`KismetMathLibrary.MakeRotationFromAxes` (`KismetMathLibrary.Normal` (`KismetMathLibrary.ProjectVectorOnToPlane` (`KismetMathLibrary.GetForwardVector` _rotation) _impactnormal_2)) (`KismetMathLibrary.Normal` (`KismetMathLibrary.ProjectVectorOnToPlane` (`KismetMathLibrary.GetRightVector` _rotation) _impactnormal_2)) _impactnormal_2)))
    (bind _output_get_2 (set `self.LinearVelocityLocal` (`KismetMathLibrary.LessLess_VectorRotator` (/ (- _returnvalue _returnvalue_2) 100.0) _output_get)))
    (set `self.IsLowSpeed` (< (`KismetMathLibrary.VSize` _output_get_2) 5.0))
    (`self.UpdateContactPatchLength`)
    (`self.UpdateSlipAngle`)
    (`self.UpdateStaticFriction`)
    (`self.UpdateSkidFriction`)
    (`self.UpdateSlidingFriction`)
    (`self.UpdateLateralForceSlipAngle`)
    (set `self.TireForceUnclamped` (+ (`self.StaticFriction`) (`KismetMathLibrary.MakeVector` (select `bool` (`self.IsLocked`) :`false` (`self.LongForce`) :`true` _slidingfriction_x_2) (select `bool` (or (`self.IsLocked`) (`self.IsLowSpeed`)) :`false` (`self.LateralForceSlipAngle`) :`true` _slidingfriction_y))))
    (set `self.Sx` (`KismetMathLibrary.SafeDivide` (.x (`self.TireForceUnclamped`)) _maxforce_2))
    (set `self.Sy` (`KismetMathLibrary.SafeDivide` (.y (`self.TireForceUnclamped`)) _maxforce_2))
    (set `self.Fx` (.x (select `bool` (> (`KismetMathLibrary.VSize` _tireforceunclamped) _maxforce) :`false` _tireforceunclamped :`true` (* (`KismetMathLibrary.Normal` _tireforceunclamped) _maxforce))))
    (set `self.Fy` (.y (select `bool` (> (`KismetMathLibrary.VSize` _tireforceunclamped) _maxforce) :`false` _tireforceunclamped :`true` (* (`KismetMathLibrary.Normal` _tireforceunclamped) _maxforce))))
    (set `self.TireFrictionForceVec` (+ (* (`KismetMathLibrary.GetForwardVector` _contactpatchrotation) (`self.Fx`)) (* (`KismetMathLibrary.GetRightVector` _contactpatchrotation) (`self.Fy`))))
    (`self.UpdateMz`)))

(fn `Trace`
  (bind _location (.location (`self.HubWorldTransform`)))
  (bind (_outhit _returnvalue) (`KismetSystemLibrary.LineTraceSingle` _location (- _location (* (`KismetMathLibrary.GetUpVector` (.rotation (`self.HubWorldTransform`))) (`self.WheelRadius`))) "TraceTypeQuery1"))
  (bind _output_get (set `self.Hit` _returnvalue))
  (if _output_get
    (bind _output_get_2 (set `self.HitResult` _outhit))
    (bind _output_get_3 (set `self.WheelRadiusEffective` (`.Distance` (`GameplayStatics.BreakHitResult` _output_get_2))))
    (set `self.Re` (* _output_get_3 0.01))
    (set `self.TireCompressZ` (- (`self.WheelRadius`) (`self.WheelRadiusEffective`)))
    (else
      (bind _output_get_4 (set `self.WheelRadiusEffective` (`self.WheelRadius`)))
      (set `self.Re` (* _output_get_4 0.01))
      (set `self.TireCompressZ` 0.0))))

(fn `Update`
  (params (InDeltaTime :type "Float (double-precision)") (InDriveTorque :type "Float (double-precision)") (InBrakeTorque :type "Float (double-precision)") (InSteeringAngle :type "Float (double-precision)") (BodyTransform :type "Transform Structure (by ref)"))
  (set `self.Delta Time` InDeltaTime)
  (set `self.DriveTorque` InDriveTorque)
  (set `self.BrakeTorque` InBrakeTorque)
  (set `self.SteeringAngle` InSteeringAngle)
  (set `self.HubWorldTransform` (`KismetMathLibrary.ComposeTransforms` (`KismetMathLibrary.MakeTransform` (.location (`self.GetRelativeTransform`)) (`KismetMathLibrary.MakeRotator` 0.0 0.0 InSteeringAngle)) BodyTransform))
  (`self.ApplyTorque`)
  (`self.Update Pitch Angle`)
  (`self.Trace`)
  (if (`self.Hit`)
    (`self.GetTireRadialForce`)
    (`self.TireModelGetForce`)
    (`self.UpdateReactionTorque`)
    (`self.ApplyForces`)
    (else
      (set `self.Sx` 0.0)
      (set `self.Sy` 0.0)
      (set `self.Fx` 0.0)
      (set `self.Fy` 0.0)
      (set `self.TireCompressZPrev` 0.0)
      (set `self.ReactionTorque` 0.0)
      (set `self.ContactPatchLength` 0.0)
      (set `self.Mz` 0.0))))

(fn `Update Pitch Angle`
  (set `self.WheelPitchAngle` (mod (+ (`self.WheelPitchAngle`) (`KismetMathLibrary.RadiansToDegrees` (* (`self.WheelAngularVelocity`) (`self.Delta Time`) -1.0))) 360.0)))

(fn `UpdateContactPatchLength`
  (bind _wheelradius (`self.WheelRadius`))
  (bind _wheelradiuseffective (`self.WheelRadiusEffective`))
  (set `self.ContactPatchLength` (* (* (`KismetMathLibrary.Sqrt` (- (* _wheelradius _wheelradius) (* _wheelradiuseffective _wheelradiuseffective))) 2.0) 0.01)))

(fn `UpdateInertia`
  (bind _returnvalue (* (`self.WheelRadius`) 0.01))
  (bind _output_get (set `self.WheelInertia` (* _returnvalue _returnvalue (`self.WheelMassTotal`) 0.5)))
  (set `self.WheelInertiaInversed` (`KismetMathLibrary.SafeDivide` 1.0 _output_get)))

(fn `UpdateLateralForceSlipAngle`
  (set `self.LateralForceSlipAngle` (* (`KismetMathLibrary.SafeDivide` (`self.SlipAngle`) (`self.SlipAnglePeak`)) (`self.MaxForce`))))

(fn `UpdateMz`
  ;[1 1 1] PT = f(SlipAngle) * CPLength * 0.167
  (set `self.PneumatickTrail` (* (`self.ContactPatchLength`) (`CurveFloat.GetFloatValue` (`self.Crv_PneumatickTrail`) (`KismetMathLibrary.Lerp` 1.0 (`KismetMathLibrary.Abs` (`self.Sy`)) (`KismetMathLibrary.MapRangeClamped` (`KismetMathLibrary.VSize` (`self.LinearVelocityLocal`)) 7.0 10.0 0.0 1.0))) 0.16667))
  (set `self.Mz` (* (`self.Fy`) (`self.PneumatickTrail`))))

(fn `UpdateReactionTorque`
  (set `self.ReactionTorque` (* (`self.Fx`) (`self.Re`) -1.0 (`KismetMathLibrary.Conv_BoolToDouble` (not (`self.IsLocked`))))))

(fn `UpdateSkidFriction`
  (set `self.LongForce` (`KismetMathLibrary.SafeDivide` (* (/ (- (`self.WheelAngularVelocity`) (`KismetMathLibrary.SafeDivide` (.x (`self.LinearVelocityLocal`)) (`self.Re`))) (`self.Delta Time`)) (`self.WheelInertia`)) (`self.Re`))))

(fn `UpdateSlidingFriction`
  (bind _linearvelocitylocal (`self.LinearVelocityLocal`))
  (bind _returnvalue (* (/ (`self.MassPerWheel`) (`self.Delta Time`)) (`KismetMathLibrary.MapRangeClamped` (`KismetMathLibrary.VSize` _linearvelocitylocal) 2.0 4.0 0.3 1.0) -1.0))
  (set `self.SlidingFriction` (* _linearvelocitylocal (`KismetMathLibrary.MakeVector` _returnvalue _returnvalue))))

(fn `UpdateSlipAngle`
  (bind (_linearvelocitylocal_x _linearvelocitylocal_y) (`KismetMathLibrary.BreakVector` (`self.LinearVelocityLocal`)))
  (set `self.SlipAngle` (`KismetMathLibrary.DegAtan2` (* _linearvelocitylocal_y -1.0) (`KismetMathLibrary.Abs` _linearvelocitylocal_x))))

(fn `UpdateStaticFriction`
  (set `self.StaticFriction` (`KismetMathLibrary.MakeVector` (* (`KismetMathLibrary.Conv_BoolToDouble` (`self.IsLocked`)) (.x (`KismetMathLibrary.LessLess_VectorRotator` (`KismetMathLibrary.MakeVector` 0.0 0.0 (* (`self.MassPerWheel`) 9.8)) (`self.ContactPatchRotation`)))) (.y (`KismetMathLibrary.LessLess_VectorRotator` (`KismetMathLibrary.MakeVector` 0.0 0.0 (* (`self.MassPerWheel`) 9.8)) (`self.ContactPatchRotation`))))))