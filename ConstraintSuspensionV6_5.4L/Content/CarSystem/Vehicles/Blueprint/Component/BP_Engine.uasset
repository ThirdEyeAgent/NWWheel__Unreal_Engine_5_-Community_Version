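; Engine component for the car system that simulates crankshaft RPM and angular velocity from throttle, load torque and starter torque.
; Update derives net torque from a vector curve (X output, absolute Y loss), adding an idle throttle that fades above idle RPM.
; Torque is integrated through inverse inertia, optionally computed from flywheel mass and diameter, with speed clamped between 70% idle and max RPM.
; AddLoadTorque applies extra load separately; ASR is only stored.
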(fn `AddLoadTorque`
  (params (LoadTorque :type "Float (double-precision)"))
  (bind _rpmtorad (`self.RPMToRad`))
  (bind _output_get (set `self.AngularVelocity` (`KismetMathLibrary.FClamp` (+ (`self.AngularVelocity`) (* LoadTorque (`self.InertiaInversed`) (`self.DeltaTime`))) (* (* (`self.IdleRPM`) 0.7) _rpmtorad) (* (`self.MaxRPM`) _rpmtorad))))
  (set `self.RPM` (* _output_get (`self.RadToRPM`))))

(fn `GetActualThrottle`)

(fn `GetAngularVelocity`
  (returns (AngularVelocity :type "Float (double-precision)"))
  (return (`self.AngularVelocity`)))

(fn `GetInertia`
  (returns (Inertia :type "Float (double-precision)"))
  (return (`self.Inertia`)))

(fn `GetNetTorque`
  (returns (NetTorque :type "Float (double-precision)"))
  (return (`self.NetTorque`)))

(fn `GetRPM`
  (returns (RPM :type "Float (double-precision)"))
  (return (`self.RPM`)))

(fn `InertiaFromFlywheel`
  (bind _returnvalue (* (`self.FlywheelDiameter`) 0.5))
  (set `self.Inertia` (* (* _returnvalue _returnvalue) (`self.FlywheelMass`) 0.5)))

(fn `Init`
  (params (InertiaFromFlywheel :type Boolean))
  (if InertiaFromFlywheel
    (`self.InertiaFromFlywheel`))
  (set `self.InertiaInversed` (`KismetMathLibrary.SafeDivide` 1.0 (`self.Inertia`)))
  (bind _output_get (set `self.RPMToRad` (/ (`KismetMathLibrary.GetPI`) 30.0)))
  (set `self.RadToRPM` (/ 1.0 _output_get)))

(fn `Update`
  (params (InDeltaTime :type "Float (double-precision)") (InThrottle :type "Float (double-precision)") (InLoadTorque :type "Float (double-precision)") (InStarterTorque :type "Float (double-precision)") (InASR :type "Float (double-precision)"))
  (set `self.DeltaTime` InDeltaTime)
  (set `self.Throttle` InThrottle)
  (set `self.LoadTorque` InLoadTorque)
  (set `self.StarterTorque` InStarterTorque)
  (set `self.ASR` InASR)
  (`self.UpdateInternal`))

(fn `UpdateInternal`
  (bind _rpmtorad (`self.RPMToRad`))
  (bind _returnvalue (`KismetMathLibrary.Abs` (.y (`CurveVector.GetVectorValue` (`self.TorqueCurve`) (`self.RPM`)))))
  (bind _returnvalue_2 (+ (.x (`CurveVector.GetVectorValue` (`self.TorqueCurve`) (`self.RPM`))) _returnvalue))
  (set `self.IdleThrottle` (* (`KismetMathLibrary.SafeDivide` _returnvalue _returnvalue_2) (`KismetMathLibrary.MapRangeClamped` (`self.RPM`) (`self.IdleRPM`) (`KismetMathLibrary.Lerp` (`self.IdleRPM`) (`self.MaxRPM`) 0.17) 1.0)))
  (set `self.ActualThrottle` (+ (`self.IdleThrottle`) (`self.Throttle`)))
  (bind _output_get (set `self.NetTorque` (- (+ (* _returnvalue_2 (`self.ActualThrottle`)) (`self.LoadTorque`) (`self.StarterTorque`)) _returnvalue)))
  (bind _output_get_2 (set `self.AngularVelocity` (`KismetMathLibrary.FClamp` (+ (`self.AngularVelocity`) (* _output_get (`self.InertiaInversed`) (`self.DeltaTime`))) (* (* (`self.IdleRPM`) 0.7) _rpmtorad) (* (`self.MaxRPM`) _rpmtorad))))
  (set `self.RPM` (* _output_get_2 (`self.RadToRPM`))))