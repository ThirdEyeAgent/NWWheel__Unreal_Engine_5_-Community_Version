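; BP_Clutch is a vehicle clutch component that computes the torque transferred between engine and drivetrain load each update.
; An automatic lock ratio rises with engine RPM over a configurable range and scales the input lock ratio.
; Torque pulls engine velocity toward an inertia-weighted common velocity with the load within one timestep, clamped to torque capacity scaled by lock.
; Getters expose the resulting torque and lock.
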(fn `GetEqualizationVelocity`
  (returns (Value :type "Float (double-precision)"))
  (bind _engineinertia (`self.EngineInertia`))
  (bind _loadinertia (`self.LoadInertia`))
  (return (`KismetMathLibrary.SafeDivide` (+ (* (`self.EngineVelocity`) _engineinertia) (* (`self.LoadVelocity`) _loadinertia)) (+ _engineinertia _loadinertia))))

(fn `GetLock`
  (returns (Value :type "Float (double-precision)"))
  (return (`self.LockRatio`)))

(fn `GetTorque`
  (returns (Value :type "Float (double-precision)"))
  (return (`self.Torque`)))

(fn `Init`
  (set `self.RadToRPM` (/ 30.0 (`KismetMathLibrary.GetPI`))))

(fn `Update`
  (params (InDeltaTime :type "Float (double-precision)") (InEngineVelocity :type "Float (double-precision)") (InEngineInertia :type "Float (double-precision)") (InLoadVelocity :type "Float (double-precision)") (InLoadInertia :type "Float (double-precision)") (InLockRatio :type "Float (double-precision)"))
  (set `self.DeltaTime` InDeltaTime)
  (set `self.EngineVelocity` InEngineVelocity)
  (set `self.EngineInertia` InEngineInertia)
  (set `self.LoadVelocity` InLoadVelocity)
  (set `self.LoadInertia` InLoadInertia)
  (set `self.LockRatioInput` InLockRatio)
  (`self.UpdateAutoLock`)
  (set `self.LockRatio` (* (`self.AutoLockRatio`) (`self.LockRatioInput`)))
  (`self.UpdateClutchTorque`))

(fn `UpdateAutoLock`
  (bind (_x _y) (`KismetMathLibrary.BreakVector2D` (`self.AutoLockMapRangeRPM`)))
  (set `self.AutoLockRatio` (`KismetMathLibrary.MapRangeClamped` (* (`self.EngineVelocity`) (`self.RadToRPM`)) _x _y 0.0 1.0)))

(fn `UpdateClutchTorque`
  (bind _returnvalue (* (`self.TorqueCapacity`) (`self.LockRatio`)))
  (bind _value (`self.GetEqualizationVelocity`))
  (set `self.Torque` (`KismetMathLibrary.FClamp` (* (/ (- _value (`self.EngineVelocity`)) (`self.DeltaTime`)) (`self.EngineInertia`)) (* _returnvalue -1.0) _returnvalue)))