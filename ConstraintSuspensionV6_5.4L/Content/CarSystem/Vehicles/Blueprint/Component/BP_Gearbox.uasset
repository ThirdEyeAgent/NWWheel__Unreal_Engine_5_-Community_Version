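; Vehicle gearbox that tracks the current gear and ratio, converting torque toward the wheels and velocity and inertia toward the engine.
; Update auto-shifts on engine RPM thresholds and, with auto reverse, uses brake at low forward speed and throttle to move between forward, zero and reverse gears.
; Index -1 selects a negated reverse ratio.
; Shifts apply immediately after index validation; the shift-delay timer exists but is never started here.
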(fn `GetGearIndex`
  (returns (Value :type Integer))
  (return (`self.GearIndex`)))

(fn `GetGearRatio`
  (returns (Value :type "Float (double-precision)"))
  (return (`self.GearRatio`)))

(fn `GetIsGearChangeInProgress`
  (returns (Value :type Boolean))
  (return (`self.IsGearChangeInProgress`)))

(fn `IndexCheck`
  (params (IndexToCheck :type Integer))
  (if (or (== IndexToCheck -1) (`KismetArrayLibrary.Array_IsValidIndex` (`self.GearRatioArray`) IndexToCheck))
    (set `self.NextGearIndex` IndexToCheck)
    (`self.ShiftGearCallback`)))

(fn `Init`)

(fn `SetNeutral`
  (set `self.GearRatio` 0.0))

(fn `ShiftGearByIndex`
  (params (Index :type Integer))
  (`self.IndexCheck` Index))

(fn `ShiftGearCallback`
  (if (== (`self.NextGearIndex`) -1)
    (set `self.GearRatio` (* (`KismetMathLibrary.Abs` (`self.ReverseGearRatio`)) -1.0))
    (else
      (set `self.GearRatio` (`|GetArrayItem` (`self.GearRatioArray`) (`self.NextGearIndex`)))))
  (set `self.GearIndex` (`self.NextGearIndex`)))

(fn `ShiftGearDown`
  (`self.IndexCheck` (- (`self.GearIndex`) 1)))

(fn `ShiftGearUp`
  (`self.IndexCheck` (+ (`self.GearIndex`) 1)))

(fn `StartTimer`
  (set `self.ElapsedTime` 0.0)
  (set `self.IsTimerActivated` true))

(fn `StopTimer`
  (set `self.IsTimerActivated` false)
  (set `self.ElapsedTime` 0.0))

(fn `ToEngine`
  (params (InVelocity :type "Float (double-precision)") (InInertia :type "Float (double-precision)"))
  (returns (OutVelocity :type "Float (double-precision)") (OutInertia :type "Float (double-precision)"))
  (bind _gearratio (`self.GearRatio`))
  (return (* InVelocity _gearratio) (`KismetMathLibrary.SafeDivide` InInertia (* _gearratio _gearratio))))

(fn `ToWheel`
  (params (InTorque :type "Float (double-precision)"))
  (returns (OutTorque :type "Float (double-precision)"))
  (return (* InTorque (`self.GearRatio`))))

(fn `Update`
  (params (InDeltaTime :type "Float (double-precision)") (InEngineRPM :type "Float (double-precision)") (InCarForwardSpeedMPS :type "Float (double-precision)") (InThrottle :type "Float (double-precision)") (InBrake :type "Float (double-precision)"))
  (bind _enginerpm (`self.EngineRPM`))
  (`|ExecutionSequence`
    (:`then_0`
      (set `self.DeltaTime` InDeltaTime)
      (set `self.EngineRPM` InEngineRPM)
      (set `self.CarForwardSpeedMPS` InCarForwardSpeedMPS)
      (set `self.ThrottleInput` InThrottle)
      (set `self.BrakeInput` InBrake)
      (`self.UpdateTimer`)
      (if (`self.IsAutoReverse`)
        _
        (else
          _))
      (if (`self.IsAutoGearShift`)
        (`self.UpdateTimer`)
        (if (`self.IsAutoReverse`)
          _
          (else
            _))
        (if (`self.IsAutoGearShift`)
          (if (> _enginerpm (`self.ShiftUpRPM`))
            (if (> (`self.GearIndex`) -1)
              (`/Engine/EditorBlueprintResources/StandardMacros.CompareInt` (`self.GearIndex`) (- (`KismetArrayLibrary.Array_Length` (`self.GearRatioArray`)) 1)
                (:`>`
                  (if (< _enginerpm (`self.ShiftDownRPM`)) :!label _label
                    (if (> (`self.GearIndex`) 1)
                      (`self.ShiftGearDown`))))
                (:`==`
                  (goto _label))
                (:`<`
                  (`self.ShiftGearUp`)))
              (else
                (goto _label)))
            (else
              (goto _label))))))
    (:`then_1`
      (if (`self.IsAutoGearShift`)
        (if (not (`self.IsGearChangeInProgress`))
          (if (< (`self.EngineRPM`) (`self.ShiftDownRPM`))
            (if (> (`self.GearIndex`) 1)
              (`self.ShiftGearDown`))))))
    (:`then_2`
      (if (`self.IsAutoReverse`)
        (if (> (`self.BrakeInput`) 0.1)
          (if (< (`self.CarForwardSpeedMPS`) 0.5)
            (if (> (`self.GearIndex`) 0)
              (`self.ShiftGearByIndex` 0)
              (elif (== (`self.GearIndex`) 0)
                (`self.ShiftGearByIndex` -1)))))))
    (:`then_3`
      (if (`self.IsAutoReverse`)
        (if (> (`self.ThrottleInput`) 0.1)
          (if (<= (`self.GearIndex`) 0)
            (`self.ShiftGearByIndex` 1)))))))

(fn `UpdateTimer`
  (if (`self.IsTimerActivated`)
    (bind _output_get (set `self.ElapsedTime` (+ (`self.ElapsedTime`) (`self.DeltaTime`))))
    (if (>= _output_get (`self.GearShiftTime`))
      (`self.StopTimer`)
      (`self.ShiftGearCallback`))))