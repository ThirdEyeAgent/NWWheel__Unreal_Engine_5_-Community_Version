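; Drivable Porsche vehicle pawn with automatic transmission, Enhanced Input controls and three switchable cameras.
; The physics-thread AdvancedTick smooths steering and runs the engine, clutch and gearbox chain, sending torque to the rear wheels, with auto-reverse on S.
; Tick updates wheel visuals, engine audio, debug readouts and third-person camera FOV and swing.
; The construction script aligns suspension top joints to their ball joints.
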(event `self.ReceiveBeginPlay`
  ;[1 1 1 1 82] Begin Play
  (set `self.Meshes` (`self.K2_GetComponentsByClass` "/Script/Engine.MeshComponent"))
  (`EnhancedInputSubsystemInterface.AddMappingContext` (pcsubsystem `EnhancedInputLocalPlayerSubsystem` (`GameplayStatics.GetPlayerController` 0)) "/Game/CarSystem/Input/IAC_CarInputMapping.IAC_CarInputMapping" 0 (struct))
  (`self.InitComponents`)
  (`self.InitRef`))

(event `self.ReceiveTick`
  (params (DeltaSeconds :type "Float (single-precision)"))
  (bind _enginesound (`self.EngineSound`))
  ;[1 1 1 1 82] Event Tick
  (set `self.Delta Seconds` DeltaSeconds)
  (`self.WakeMesh`)
  (`self.UpdateVisualWheels`)
  (`self.UpdateCamera`)
  (set `self.ThrottleInterp` (`/Game/CarSystem/Vehicles/Blueprint/Component/BP_Engine.ActualThrottle` (`self.BP_Engine`)))
  (`AudioParameterControllerInterface.SetFloatParameter` _enginesound "RPM" (`/Game/CarSystem/Vehicles/Blueprint/Component/BP_Engine.RPM` (`self.BP_Engine`)))
  (`AudioParameterControllerInterface.SetFloatParameter` _enginesound "Load" (`self.ThrottleInterp`))
  (`self.PrintValues`)
  (`self.CameraInput`))

(event `EnhancedInput|/Game/CarSystem/Input/IA_Steering`
  (params (ActionValue :type "Float (double-precision)") (ElapsedSeconds :type "Float (double-precision)") (TriggeredSeconds :type "Float (double-precision)") (InputAction :type "InputAction Object Reference" :default "/Game/CarSystem/Input/IA_Steering.IA_Steering"))
  ;[1 1 1 1 82] steering
  (:`Triggered`
    (set `self.SteeringInput` ActionValue :!label _label))
  (:`Canceled`
    (goto _label))
  (:`Completed`
    (goto _label)))

(event `EnhancedInput|/Game/CarSystem/Input/IA_GearUp`
  (params (ActionValue :type Boolean) (ElapsedSeconds :type "Float (double-precision)") (TriggeredSeconds :type "Float (double-precision)") (InputAction :type "InputAction Object Reference" :default "/Game/CarSystem/Input/IA_GearUp.IA_GearUp"))
  ;[1 1 1 1 82] Manual Gear Shift
  (:`Started`
    (`/Game/CarSystem/Vehicles/Blueprint/Component/BP_Gearbox.ShiftGearUp` (`self.BP_Gearbox`))))

(event `EnhancedInput|/Game/CarSystem/Input/IA_Throttle`
  (params (ActionValue :type "Float (double-precision)") (ElapsedSeconds :type "Float (double-precision)") (TriggeredSeconds :type "Float (double-precision)") (InputAction :type "InputAction Object Reference" :default "/Game/CarSystem/Input/IA_Throttle.IA_Throttle"))
  ;[1 1 1 1 82] Throttle
  (:`Triggered`
    (set `self.ThrottleInput` ActionValue :!label _label_2))
  (:`Canceled`
    (goto _label_2))
  (:`Completed`
    (goto _label_2)))

(event `EnhancedInput|/Game/CarSystem/Input/IA_GearDown`
  (params (ActionValue :type Boolean) (ElapsedSeconds :type "Float (double-precision)") (TriggeredSeconds :type "Float (double-precision)") (InputAction :type "InputAction Object Reference" :default "/Game/CarSystem/Input/IA_GearDown.IA_GearDown"))
  ;[1 1 1 1 82] Manual Gear Shift
  (:`Started`
    (`/Game/CarSystem/Vehicles/Blueprint/Component/BP_Gearbox.ShiftGearDown` (`self.BP_Gearbox`))))

(event `EnhancedInput|/Game/CarSystem/Input/IA_Brake`
  (params (ActionValue :type "Float (double-precision)") (ElapsedSeconds :type "Float (double-precision)") (TriggeredSeconds :type "Float (double-precision)") (InputAction :type "InputAction Object Reference" :default "/Game/CarSystem/Input/IA_Brake.IA_Brake"))
  ;[1 1 1 1 82] Throttle
  (:`Triggered`
    (set `self.BrakeInput` ActionValue :!label _label_3))
  (:`Canceled`
    (goto _label_3))
  (:`Completed`
    (goto _label_3)))

(event `EnhancedInput|/Game/CarSystem/Input/IA_ViewChange`
  (params (ActionValue :type Boolean) (ElapsedSeconds :type "Float (double-precision)") (TriggeredSeconds :type "Float (double-precision)") (InputAction :type "InputAction Object Reference" :default "/Game/CarSystem/Input/IA_ViewChange.IA_ViewChange"))
  ;[1 1 1 1 82] Camera System
  (:`Completed`
    (`ActorComponent.SetActive` (`self.HoodCamera`) false false)
    (`ActorComponent.SetActive` (`self.FirstPersonCamera`) false false)
    (`ActorComponent.SetActive` (`self.ThirdPersonCamera`) false false)
    (switch `int` (`self.CameraIndex`)
      (:`0`
        (set `self.CameraIndex` 1))
      (:`1`
        (set `self.CameraIndex` 2))
      (:`2`
        (set `self.CameraIndex` 0)))
    (`ActorComponent.SetActive` (select `int` (`self.CameraIndex`) :`0` (`self.ThirdPersonCamera`) :`1` (`self.FirstPersonCamera`) :`2` (`self.HoodCamera`) :!type "ActorComponent Object Reference") true false)))

(event `Key|LeftShift`
  (params (Key :type "Key Structure"))
  ;[1 1 1 1 81] Front ABS Brake
  (:`Pressed`
    (set `self.FrontBrakeInput` 1.0))
  (:`Released`
    (set `self.FrontBrakeInput` 0.0)))

(event `Key|SpaceBar`
  (params (Key :type "Key Structure"))
  ;[1 1 1 1 74] handbrake
  (:`Pressed`
    (set `self.HandbrakeInput` 1.0))
  (:`Released`
    (set `self.HandbrakeInput` 0.0)))

(event `self.AdvancedTick`
  (params (DeltaTime :type "Float (single-precision)") (SimTime :type "Float (single-precision)"))
  (bind _returnvalue (== (`/Game/CarSystem/Vehicles/Blueprint/Component/BP_Gearbox.GetGearIndex` (`self.BP_Gearbox`)) -1))
  ;[1 1 1] physic thread
  (set `self.PhysicDeltaTime` DeltaTime)
  (`self.UpdateSteering`)
  (`self.UpdateTransmission`)
  (if (`self.IsReverseRequested`)
    (if (not _returnvalue)
      (if (< (`KismetMathLibrary.VSize` (`self.GetVelocity`)) 300.0)
        (`/Game/CarSystem/Vehicles/Blueprint/Component/BP_Gearbox.ShiftGearByIndex` (`self.BP_Gearbox`) -5)
        (set `self.IsReverseRequested` false)
        (else
          (set `self.BrakeInput` 1.0)))
      (else
        (set `self.ThrottleInput` 1.0)))
    (elif _returnvalue
      (if (== (`self.BrakeInput`) 1.0)
        (set `self.BrakeInput` 0.0)))))

(event `Key|S`
  (params (Key :type "Key Structure"))
  (bind _bp_gearbox (`self.BP_Gearbox`))
  ;[1 1 1 1 90] Auto Reverse
  (:`Pressed`
    (set `self.IsReverseRequested` true)
    (`/Game/CarSystem/Vehicles/Blueprint/Component/BP_Gearbox.ShiftGearByIndex` (`self.BP_Gearbox`) -1))
  (:`Released`
    (set `self.IsReverseRequested` false)
    (if (== (`/Game/CarSystem/Vehicles/Blueprint/Component/BP_Gearbox.GetGearIndex` _bp_gearbox) -1)
      (`/Game/CarSystem/Vehicles/Blueprint/Component/BP_Gearbox.ShiftGearByIndex` _bp_gearbox 0)
      (set `self.ThrottleInput` 0.0))))

(fn `CameraInput`
  (bind _springarm (`self.SpringArm`))
  (bind _bp_engine (`self.BP_Engine`))
  (bind _nettorque (`/Game/CarSystem/Vehicles/Blueprint/Component/BP_Engine.GetNetTorque` _bp_engine))
  (switch `int` (`self.CameraIndex`)
    (:`0`
      (if (> _nettorque 1000.0)
        (`CameraComponent.SetFieldOfView` (`self.ThirdPersonCamera`) (`KismetMathLibrary.MapRangeClamped` _nettorque 0.0 1000.0 90.0 110.0))
        (else
          (`CameraComponent.SetFieldOfView` (`self.ThirdPersonCamera`) (`KismetMathLibrary.MapRangeClamped` (`/Game/CarSystem/Vehicles/Blueprint/Component/BP_Engine.RPM` _bp_engine) 7000.0 100.0 110.0 90.0))))
      (if (> (`self.ThrottleInput`) 0.0)
        (`SceneComponent.K2_SetRelativeRotation` _springarm (`KismetMathLibrary.RInterpTo` (`SceneComponent.RelativeRotation` _springarm) (`KismetMathLibrary.MakeRotator` 0.0 -6.0 (`KismetMathLibrary.FClamp` (* (`self.SteeringAngle`) (`KismetMathLibrary.MapRangeClamped` (`/Game/CarSystem/Vehicles/Blueprint/Component/BP_Engine.GetNetTorque` (`self.BP_Engine`)) 10.0 1000.0 1.0 0.5)) -45.0 45.0)) (`GameplayStatics.GetWorldDeltaSeconds`) 3.0) false false)))))

(fn `InitComponents`
  (`/Game/CarSystem/Vehicles/Blueprint/Component/BP_Wheel.SetBody` (`self.PRT_Wheel_0`) (`self.Hub_0_Center`))
  (`/Game/CarSystem/Vehicles/Blueprint/Component/BP_Wheel.SetBody` (`self.PRT_Wheel_1`) (`self.Hub_1_Center`))
  (`/Game/CarSystem/Vehicles/Blueprint/Component/BP_Wheel.SetBody` (`self.PRT_Wheel_2`) (`self.Hub_2_Center`))
  (`/Game/CarSystem/Vehicles/Blueprint/Component/BP_Wheel.SetBody` (`self.PRT_Wheel_3`) (`self.Hub_3_Center`))
  (`/Game/CarSystem/Vehicles/Blueprint/Component/BP_Engine.Init` (`self.BP_Engine`) false)
  (`/Game/CarSystem/Vehicles/Blueprint/Component/BP_Clutch.Init` (`self.BP_Clutch`))
  (`/Game/CarSystem/Vehicles/Blueprint/Component/BP_Gearbox.Init` (`self.BP_Gearbox`)))

(fn `InitRef`
  (set `self.PRT_Wheel` (`|MakeArray` (`self.PRT_Wheel_0`) (`self.PRT_Wheel_1`) (`self.PRT_Wheel_2`) (`self.PRT_Wheel_3`)))
  (set `self.WheelMesh` (`|MakeArray` (`self.Wheel_FL`) (`self.Wheel_FR`) (`self.Wheel_RL`) (`self.Wheel_RR`))))

(fn `PrintValues`
  (bind _bp_gearbox (`self.BP_Gearbox`))
  (`KismetSystemLibrary.PrintString` (`KismetStringLibrary.Concat_StrStr` "Engine RPM = " (`KismetStringLibrary.Conv_DoubleToString` (`/Game/CarSystem/Vehicles/Blueprint/Component/BP_Engine.GetRPM` (`self.BP_Engine`)))) true false (struct :`R` 1.0 :`B` 0.031044 :`A` 1.0) 0.0)
  (`KismetSystemLibrary.PrintString` (`KismetStringLibrary.Concat_StrStr` "Engine Net Torque = " (`KismetStringLibrary.Conv_DoubleToString` (`/Game/CarSystem/Vehicles/Blueprint/Component/BP_Engine.GetNetTorque` (`self.BP_Engine`)))) true false (struct :`R` 1.0 :`B` 0.031044 :`A` 1.0) 0.0)
  (`KismetSystemLibrary.PrintString` (`KismetStringLibrary.Concat_StrStr` "Clutch Torque = " (`KismetStringLibrary.Conv_DoubleToString` (`/Game/CarSystem/Vehicles/Blueprint/Component/BP_Clutch.GetTorque` (`self.BP_Clutch`)))) true false (struct :`R` 1.0 :`G` 0.604231 :`A` 1.0) 0.0)
  (`KismetSystemLibrary.PrintString` (`KismetStringLibrary.Concat_StrStr` "Gear Index = " (`KismetStringLibrary.Conv_IntToString` (`/Game/CarSystem/Vehicles/Blueprint/Component/BP_Gearbox.GetGearIndex` _bp_gearbox))) true false (struct :`G` 1.0 :`B` 0.019595 :`A` 1.0) 0.0)
  (`KismetSystemLibrary.PrintString` (`KismetStringLibrary.Concat_StrStr` "Gear Index = " (`KismetStringLibrary.Conv_DoubleToString` (`/Game/CarSystem/Vehicles/Blueprint/Component/BP_Gearbox.GetGearRatio` _bp_gearbox))) true false (struct :`G` 1.0 :`B` 0.019595 :`A` 1.0) 0.0)
  (`KismetSystemLibrary.PrintString` (`KismetStringLibrary.Concat_StrStr` "Drive Torque = " (`KismetStringLibrary.Conv_DoubleToString` (`self.NewVar`))) true false (struct :`G` 0.972917 :`B` 1.0 :`A` 1.0) 0.0))

(fn `UpdateCamera`
  (bind _springarm (`self.SpringArm`))
  (`SceneComponent.K2_SetRelativeRotation` _springarm (`KismetMathLibrary.MakeRotator` 0.0 (`KismetMathLibrary.FClamp` (+ (.pitch (`SceneComponent.RelativeRotation` _springarm)) (`self.GetInputAxisKeyValue`)) -70.0 70.0) (+ (.yaw (`SceneComponent.RelativeRotation` _springarm)) (`self.GetInputAxisKeyValue`))) false false))

(fn `UpdateSteering`
  (bind _steeringinput (`self.SteeringInput`))
  (bind _physicdeltatime (`self.PhysicDeltaTime`))
  (bind _output_get (set `self.SteeringInterp` (`KismetMathLibrary.FInterpTo` (`self.SteeringInterp`) _steeringinput _physicdeltatime (* (/ 1.0 _physicdeltatime) (select `bool` (== _steeringinput 0.0) :`false` 0.03 :`true` 0.1)))))
  (set `self.SteeringAngle` (* _output_get (`self.MaxSteeringAngle`))))

(fn `UpdateTransmission`
  (locals (DriveTorque :type "Float (double-precision)"))
  (bind _prt_wheel_2 (`self.PRT_Wheel_2`))
  (bind _prt_wheel_3 (`self.PRT_Wheel_3`))
  (bind _finalgearratio (`self.FinalGearRatio`))
  (bind _bp_clutch (`self.BP_Clutch`))
  (bind _bp_engine (`self.BP_Engine`))
  (bind _bp_engine_2 (`self.BP_Engine`))
  (bind _value (`/Game/CarSystem/Vehicles/Blueprint/Component/BP_Clutch.GetTorque` _bp_clutch))
  (bind _returnvalue (* (`self.HandbrakeInput`) 5000.0))
  (bind _returnvalue_2 (* (`self.FrontBrakeInput`) 5000.0))
  (bind _returnvalue_3 (* (`local.DriveTorque`) 0.5))
  (bind _returnvalue_4 (`PrimitiveComponent.GetPhysicsLinearVelocity` (`self.Chassis`) "None"))
  (`/Game/CarSystem/Vehicles/Blueprint/Component/BP_Gearbox.Update` (`self.BP_Gearbox`) (`self.PhysicDeltaTime`) (`/Game/CarSystem/Vehicles/Blueprint/Component/BP_Engine.GetRPM` (`self.BP_Engine`)) (/ (`KismetMathLibrary.VSize` _returnvalue_4) 100.0) (`self.ThrottleInput`) (`self.BrakeInput`))
  (bind (_outvelocity _outinertia) (`/Game/CarSystem/Vehicles/Blueprint/Component/BP_Gearbox.ToEngine` (`self.BP_Gearbox`) (* (* (+ (`/Game/CarSystem/Vehicles/Blueprint/Component/BP_Wheel.GetWheelAngularVelocity` _prt_wheel_2) (`/Game/CarSystem/Vehicles/Blueprint/Component/BP_Wheel.GetWheelAngularVelocity` _prt_wheel_3)) 0.5) (`self.FinalGearRatio`)) (`KismetMathLibrary.SafeDivide` (+ (`/Game/CarSystem/Vehicles/Blueprint/Component/BP_Wheel.GetWheelInertia` _prt_wheel_2) (`/Game/CarSystem/Vehicles/Blueprint/Component/BP_Wheel.GetWheelInertia` _prt_wheel_3)) (* _finalgearratio _finalgearratio))))
  (`/Game/CarSystem/Vehicles/Blueprint/Component/BP_Clutch.Update` _bp_clutch (`self.PhysicDeltaTime`) (`/Game/CarSystem/Vehicles/Blueprint/Component/BP_Engine.GetAngularVelocity` _bp_engine) (`/Game/CarSystem/Vehicles/Blueprint/Component/BP_Engine.Inertia` _bp_engine) _outvelocity _outinertia 1.0)
  (`/Game/CarSystem/Vehicles/Blueprint/Component/BP_Engine.Update` _bp_engine_2 (`self.PhysicDeltaTime`) (`self.ThrottleInput`) 0.0 0.0 1.0)
  (`/Game/CarSystem/Vehicles/Blueprint/Component/BP_Engine.AddLoadTorque` _bp_engine_2 _value)
  (bind _outtorque (`/Game/CarSystem/Vehicles/Blueprint/Component/BP_Gearbox.ToWheel` (`self.BP_Gearbox`) (* _value -1.0)))
  (bind _returnvalue_5 (* _outtorque (`self.FinalGearRatio`)))
  (set `local.DriveTorque` _returnvalue_5)
  (set `self.NewVar` _returnvalue_5)
  (`/Game/CarSystem/Vehicles/Blueprint/Component/BP_Wheel.Update` (`self.PRT_Wheel_0`) (`self.PhysicDeltaTime`) 0.0 _returnvalue_2 (`self.SteeringAngle`) (`self.GetPrimitiveWorldTransform` (`self.Hub_0_Center`)))
  (`/Game/CarSystem/Vehicles/Blueprint/Component/BP_Wheel.Update` (`self.PRT_Wheel_1`) (`self.PhysicDeltaTime`) 0.0 _returnvalue_2 (`self.SteeringAngle`) (`self.GetPrimitiveWorldTransform` (`self.Hub_1_Center`)))
  (`/Game/CarSystem/Vehicles/Blueprint/Component/BP_Wheel.Update` (`self.PRT_Wheel_2`) (`self.PhysicDeltaTime`) _returnvalue_3 _returnvalue 0.0 (`self.GetPrimitiveWorldTransform` (`self.Hub_2_Center`)))
  (`/Game/CarSystem/Vehicles/Blueprint/Component/BP_Wheel.Update` (`self.PRT_Wheel_3`) (`self.PhysicDeltaTime`) _returnvalue_3 _returnvalue 0.0 (`self.GetPrimitiveWorldTransform` (`self.Hub_3_Center`))))

(fn `UpdateVisualWheels`
  (bind _wheelmesh (`self.WheelMesh`))
  (for (_array_element _array_index) (`self.PRT_Wheel`)
    (if (`KismetArrayLibrary.Array_IsValidIndex` _wheelmesh _array_index)
      (`SceneComponent.K2_SetRelativeRotation` (`|GetArrayItem` _wheelmesh _array_index) (`KismetMathLibrary.ComposeRotators` (`KismetMathLibrary.RotatorFromAxisAndAngle` (0.0 -1.0 0.0) (`/Game/CarSystem/Vehicles/Blueprint/Component/BP_Wheel.GetWheelPitchAngle` _array_element)) (`KismetMathLibrary.MakeRotator` 0.0 0.0 (`/Game/CarSystem/Vehicles/Blueprint/Component/BP_Wheel.GetWheelSteeringAngle` _array_element))) false false))))

(fn `UserConstructionScript`
  (bind _returnvalue (`KismetMathLibrary.Normal` (`KismetMathLibrary.Normal` (- (`SceneComponent.K2_GetComponentLocation` (`self.JointTop_0`)) (`SceneComponent.K2_GetComponentLocation` (`self.BallJoint_0`))))))
  (bind _returnvalue_2 (`KismetMathLibrary.Normal` (`KismetMathLibrary.Normal` (- (`SceneComponent.K2_GetComponentLocation` (`self.JointTop_1`)) (`SceneComponent.K2_GetComponentLocation` (`self.BallJoint_1`))))))
  (bind _returnvalue_3 (`KismetMathLibrary.Normal` (`KismetMathLibrary.Normal` (- (`SceneComponent.K2_GetComponentLocation` (`self.JointTop_3`)) (`SceneComponent.K2_GetComponentLocation` (`self.BallJoint_3`))))))
  (bind _returnvalue_4 (`KismetMathLibrary.Normal` (`KismetMathLibrary.Normal` (- (`SceneComponent.K2_GetComponentLocation` (`self.JointTop_2`)) (`SceneComponent.K2_GetComponentLocation` (`self.BallJoint_2`))))))
  (`SceneComponent.K2_SetWorldRotation` (`self.JointTop_0`) (`KismetMathLibrary.MakeRotFromZY` _returnvalue (`KismetMathLibrary.Normal` (`KismetMathLibrary.Cross_VectorVector` (-1.0 0.0 0.0) _returnvalue))) false false)
  (`SceneComponent.K2_SetWorldRotation` (`self.JointTop_1`) (`KismetMathLibrary.MakeRotFromZY` _returnvalue_2 (`KismetMathLibrary.Normal` (`KismetMathLibrary.Cross_VectorVector` (-1.0 0.0 0.0) _returnvalue_2))) false false)
  (`SceneComponent.K2_SetWorldRotation` (`self.JointTop_2`) (`KismetMathLibrary.MakeRotFromZY` _returnvalue_4 (`KismetMathLibrary.Normal` (`KismetMathLibrary.Cross_VectorVector` (-1.0 0.0 0.0) _returnvalue_4))) false false)
  (`SceneComponent.K2_SetWorldRotation` (`self.JointTop_3`) (`KismetMathLibrary.MakeRotFromZY` _returnvalue_3 (`KismetMathLibrary.Normal` (`KismetMathLibrary.Cross_VectorVector` (-1.0 0.0 0.0) _returnvalue_3))) false false))

(fn `WakeMesh`
  (for _array_element (`self.Meshes`)
    (`PrimitiveComponent.WakeRigidBody` _array_element "None")))