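; Test actor in the car system, apparently for vehicle suspension, that auto-aligns a physics constraint to a joint.
; The construction script rotates PhysicsConstraint2 so its Z axis points at JointBall, deriving Y from that direction crossed with world X.
; BeginPlay prints the constraint's resulting relative rotation on screen for debugging.
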(event `self.ReceiveBeginPlay`
  (`KismetSystemLibrary.PrintString` (`KismetStringLibrary.Conv_RotatorToString` (`SceneComponent.RelativeRotation` (`self.PhysicsConstraint2`))) true false (struct :`G` 0.66 :`B` 1.0 :`A` 1.0) 5.0))

(fn `UserConstructionScript`
  (bind _returnvalue (`KismetMathLibrary.Normal` (`KismetMathLibrary.Normal` (- (`SceneComponent.K2_GetComponentLocation` (`self.Joint_Ball`)) (`SceneComponent.K2_GetComponentLocation` (`self.PhysicsConstraint2`))))))
  (`SceneComponent.K2_SetWorldRotation` (`self.PhysicsConstraint2`) (`KismetMathLibrary.MakeRotFromZY` _returnvalue (`KismetMathLibrary.Normal` (`KismetMathLibrary.Cross_VectorVector` _returnvalue (1.0 0.0 0.0)))) false false))